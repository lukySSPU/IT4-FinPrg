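; Player character for a game with portals, using Enhanced Input for movement relative to control yaw and for look.
; Each tick scales max walk speed by the actor's X scale, based on the speed cached at BeginPlay.
; SmoothOrientation fixes tilt after a portal: if roll is non-zero, a timeline eases control roll to zero and the capsule back to zero rotation.
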(event `self.ReceiveBeginPlay`
  (`self.Setup Input`)
  (set `self.MaxSpeed` (`CharacterMovementComponent.MaxWalkSpeed` (`self.CharacterMovement`))))

(event `EnhancedInput|/Game/Input/IA_Forward`
  (params (ActionValue :type "Float (double-precision)") (ElapsedSeconds :type "Float (double-precision)") (TriggeredSeconds :type "Float (double-precision)") (InputAction :type "InputAction Object Reference" :default "/Game/Input/IA_Forward.IA_Forward"))
  (bind (_returnvalue_roll _returnvalue_pitch _returnvalue_yaw) (`KismetMathLibrary.BreakRotator` (`self.GetControlRotation`)))
  (:`Triggered`
    (`self.AddMovementInput` (`KismetMathLibrary.GetForwardVector` (`KismetMathLibrary.MakeRotator` 0.0 0.0 _returnvalue_yaw)) ActionValue)))

(event `EnhancedInput|/Game/Input/IA_Right`
  (params (ActionValue :type "Float (double-precision)") (ElapsedSeconds :type "Float (double-precision)") (TriggeredSeconds :type "Float (double-precision)") (InputAction :type "InputAction Object Reference" :default "/Game/Input/IA_Right.IA_Right"))
  (bind (_returnvalue_roll _returnvalue_pitch _returnvalue_yaw) (`KismetMathLibrary.BreakRotator` (`self.GetControlRotation`)))
  (:`Triggered`
    (`self.AddMovementInput` (`KismetMathLibrary.GetRightVector` (`KismetMathLibrary.MakeRotator` 0.0 0.0 _returnvalue_yaw)) ActionValue)))

(event `EnhancedInput|/Game/Input/IA_Turn`
  (params (ActionValue :type "Float (double-precision)") (ElapsedSeconds :type "Float (double-precision)") (TriggeredSeconds :type "Float (double-precision)") (InputAction :type "InputAction Object Reference" :default "/Game/Input/IA_Turn.IA_Turn"))
  (:`Triggered`
    (`self.AddControllerYawInput` ActionValue)))

(event `EnhancedInput|/Game/Input/IA_LookUp`
  (params (ActionValue :type "Float (double-precision)") (ElapsedSeconds :type "Float (double-precision)") (TriggeredSeconds :type "Float (double-precision)") (InputAction :type "InputAction Object Reference" :default "/Game/Input/IA_LookUp.IA_LookUp"))
  (:`Triggered`
    (`self.AddControllerPitchInput` ActionValue)))

(event `self.ReceiveTick`
  (params (DeltaSeconds :type "Float (single-precision)"))
  (bind (_returnvalue_location _returnvalue_rotation _returnvalue_scale) (`KismetMathLibrary.BreakTransform` (`self.GetTransform` self)))
  ;[0.2686 0.7879 1 0.5] Set walk speed according to scale
  (set `CharacterMovementComponent.MaxWalkSpeed` (* (.x _returnvalue_scale) (`self.MaxSpeed`)) (`self.CharacterMovement`)))

(event `SmoothOrientation`
  (params (NewControllerRotation :type "Rotator Structure"))
  (bind _initialcontrolrotation (`self.InitialControlRotation`))
  ;[1 0.5144 0.9563 0.5] Fix player rotation after passing a tilted  portal
  (if (or (!= (.roll (`Controller.GetControlRotation` (`GameplayStatics.GetPlayerController` 0))) 0.0) (!= (.roll (`SceneComponent.K2_GetComponentRotation` (`self.CapsuleComponent`))) 0.0))
    (set `self.InitialControlRotation` (`Controller.GetControlRotation` (`GameplayStatics.GetPlayerController` 0)))
    (set `self.InitialWorldRotation` (`SceneComponent.K2_GetComponentRotation` (`self.CapsuleComponent`)))
    (bind (_direction _alpha) (`Timeline|Rotate` :!via `PlayFromStart`)
      (:`Update`
        (`Controller.SetControlRotation` (`GameplayStatics.GetPlayerController` 0) (`|EaseFunction` "EaseOut" _alpha _initialcontrolrotation (`KismetMathLibrary.MakeRotator` 0.0 (.pitch _initialcontrolrotation) (.yaw _initialcontrolrotation))))
        (`SceneComponent.K2_SetWorldRotation` (`self.CapsuleComponent`) (`|EaseFunction` "EaseOut" _alpha (`self.InitialWorldRotation`) (`KismetMathLibrary.MakeRotator` 0.0)) false false)))))

(fn `Setup Input`
  (`EnhancedInputSubsystemInterface.AddMappingContext` (pcsubsystem `EnhancedInputLocalPlayerSubsystem` (`GameplayStatics.GetPlayerController` 0)) "/Game/Input/IM_Input.IM_Input" 0 (struct)))

(fn `UserConstructionScript`)